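; BP_Screen is an in-world screen actor that displays hints and plays their audio.
; SetHint looks up the hint in DT_Hint, pushes text and texture to W_ScreenWidget, and async-loads the soft-referenced SoundCue, stopping audio if invalid.
; When audio finishes, it broadcasts HintAudioFinished for the Level Blueprint, then replays it after a retriggerable delay unless already playing.
; SetContent switches widget content, while NextHint and PreviousHint step through hints for debugging.
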(event OnAudioFinished(Audio)
  (bind _audio (Variables|Default|GetAudio))
  (Default|CallHintAudioFinished (Variables|Default|GetCurrentHint)) ; Notify Level BP
  (Utilities|FlowControl|RetriggerableDelay 5.0)
  (if (not (Audio|Components|Audio|IsPlaying _audio))
    (Audio|Components|Audio|Play _audio 0.0)))

(event Custom|SetHint
  (params (Hint :type Integer))
  (bind _audio (Variables|Default|GetAudio))
  (Variables|Default|SetCurrentHint Hint)
  (bind _returnvalue (Utilities|GetDataTableRow "/Game/DesignTest/Blueprints/Utilities/DT_Hint.DT_Hint" (Utilities|String|StringToName (Utilities|String|ToString(Integer) (Variables|Default|GetCurrentHint))))
    (:then
      (bind _output_get (Variables|Default|SetHint _returnvalue))
      (Utilities|FlowControl|Sequence
        (:then_0
          (Default|SetHint (Variables|Default|GetScreenWidget) (.hint _output_get) (.texture _output_get)))
        (:then_1
          ;[1 1 1] Handle Sounds
          (bind _object (Utilities|AsyncLoad (.sound _output_get))
            (:NotValid
              (CallFunction|StopSound :!label _label)
              (Debug|PrintWarning "Hint Sound not valid!"))
            (:Completed
              (bind _assound_cue (Utilities|Casting|CastToSoundCue _object)
                (:then
                  (Audio|Components|Audio|SetSound _audio _assound_cue)
                  (Audio|Components|Audio|Play _audio 0.0))
                (:CastFailed
                  (goto _label))))))))
    (:RowNotFound
      (Debug|PrintWarning "Hint details doesnt exist!"))))

(event EventBeginPlay
  (Variables|Default|SetScreenWidget (.AsW%20Screen%20Widget (Utilities|Casting|CastToW_ScreenWidget (UserInterface|GetUserWidgetObject (Variables|Default|GetWidget))))))

(fn ConstructionScript)

(fn NextHint
  (bind _result (Math|Integer|IncrementInt (Variables|Default|GetCurrentHint))
    (:%20%20
      (CallFunction|SetHint _result))))

(fn PreviousHint
  (bind _result (Math|Integer|DecrementInt (Variables|Default|GetCurrentHint))
    (:%20%20
      (CallFunction|SetHint _result))))

(fn PrintWarning
  (params (Warning :type String))
  (Development|PrintString (Utilities|String|Append "Warning:: " Warning) true true "(R=1.000000,G=0.963622,B=0.000000,A=1.000000)"))

(fn StopSound
  (bind _audio (Variables|Default|GetAudio))
  (Audio|Components|Audio|Stop _audio)
  (Audio|Components|Audio|SetSound _audio 0))

(fn SetContent
  (params (Index :type Integer))
  (Default|SwitchContent (Variables|Default|GetScreenWidget) Index))