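; BP_Button is a pressable button actor that reports when its Button component has been displaced far enough.
; It records the component's starting world location on BeginPlay and compares the squared distance from it against TravelDistance each Tick, avoiding a square root.
; A DoOnce fires the ButtonPressed dispatcher, intended for the Level Blueprint, and resets once the button moves back within range.
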(event EventBeginPlay
  (Variables|Default|SetInitialLocation (Transformation|GetWorldLocation (Variables|Default|GetButton))))

(event EventTick
  (params (DeltaSeconds :type Float%20%28single-precision%29))
  (if (>= (Class|KismetMathLibrary|VectorDistanceSquared (Transformation|GetWorldLocation (Variables|Default|GetButton)) (Variables|Default|GetInitialLocation)) (Variables|Default|GetTravelDistance))
    (Utilities|FlowControl|DoOnce false :!label _label
      (:Completed
        (Default|CallButtonPressed) ; Notify Level BP
      ))
    (else
      (goto _label Reset))))

(fn ConstructionScript)